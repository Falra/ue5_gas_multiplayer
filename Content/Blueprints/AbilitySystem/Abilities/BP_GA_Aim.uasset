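; BP_GA_Aim is a gameplay ability that applies an aim camera modifier to the player's camera while aiming.
; On activation it adds the modifier through the PlayerCameraManager and stores the handle, ending immediately if there is no valid player controller.
; It stays active until an Event.Combat.Aim.Ended gameplay event arrives, then ends and removes the modifier on end.
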(event `self.K2_ActivateAbility`
  (bind (_owneractor _avataractor _playercontroller) (break `GameplayAbilityActorInfo` (`self.GetActorInfo`)))
  (`/Engine/EditorBlueprintResources/StandardMacros.IsValid` _playercontroller
    (:`Is Valid`
      (bind _returnvalue (`PlayerCameraManager.AddNewCameraModifier` (`PlayerController.PlayerCameraManager` _playercontroller) "/Game/CameraModifiers/AimCameraModifier.AimCameraModifier_C"))
      (set `self.AimModifierHandle` _returnvalue)
      (`AbilityTask_WaitGameplayEvent.WaitGameplayEvent` (struct :`TagName` "Event.Combat.Aim.Ended") null
        (:`EventReceived`
          (`self.K2_EndAbility`))))
    (:`Is Not Valid`
      (`self.K2_EndAbility`))))

(event `self.K2_OnEndAbility`
  (params (bWasCancelled :type Boolean))
  (bind (_owneractor _avataractor _playercontroller) (break `GameplayAbilityActorInfo` (`self.GetActorInfo`)))
  (`/Engine/EditorBlueprintResources/StandardMacros.IsValid` _playercontroller
    (:`Is Valid`
      (`PlayerCameraManager.RemoveCameraModifier` (`PlayerController.PlayerCameraManager` _playercontroller) (`self.AimModifierHandle`)))))