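; Gameplay ability for a projectile weapon shot that fires a rocket from the equipped weapon.
; On activation it traces from the weapon toward the focus point over the shooting distance and passes the hit to the weapon's effects.
; It then launches the rocket projectile just ahead of the muzzle, offset and oriented along the trace direction, with the character as owner and instigator, and ends immediately.
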(event `self.K2_ActivateAbility`
  (bind _returnvalue (`self.GetActionGameCharacterFromActorInfo`))
  (bind (_bblockinghit _binitialoverlap _time _distance _location _impactpoint _normal _impactnormal _physmat _hitactor _hitcomponent _hitbonename _bonename _hititem _elementindex _faceindex _tracestart _traceend) (`GameplayStatics.BreakHitResult` (`self.GetWeaponToFocusTraceResult` (`self.ShootingDistance`) "TraceTypeQuery3")))
  (bind _returnvalue_2 (`KismetMathLibrary.Normal` (- _traceend _tracestart)))
  (`WeaponItemActor.PlayWeaponEffects` (`self.GetEquippedWeaponItemActor`) (`GameplayStatics.MakeHitResult` _bblockinghit _binitialoverlap _time _distance _location _impactpoint _normal _impactnormal null null null "None" "None" 0 0 0 _tracestart _traceend))
  (`ActionGameStatics.LaunchProjectile` "/Game/Blueprints/Projectiles/Rocket.Rocket_C" (`KismetMathLibrary.MakeTransform` (+ (`WeaponItemActor.GetMuzzleLocation` (`self.GetEquippedWeaponItemActor`)) (* _returnvalue_2 (`self.SpawnOffset`))) (`KismetMathLibrary.Conv_VectorToRotator` _returnvalue_2)) _returnvalue _returnvalue)
  (`self.K2_EndAbility`))