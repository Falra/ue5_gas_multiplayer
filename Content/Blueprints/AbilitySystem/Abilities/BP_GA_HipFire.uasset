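; Gameplay ability for automatic hip fire with the equipped weapon, started by a gameplay event.
; It plays the weapon's attack montage and fires immediately, then on a looping timer at the weapon's fire rate.
; Each shot line-traces from the muzzle along control rotation, applying the damage effect through the hit actor's ability system.
; The attack-ended event or montage completion, interruption or cancellation ends the ability, clearing the timer.
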(event `self.K2_ActivateAbilityFromEvent`
  (params (EventData :type "GameplayEventData Structure (by ref)"))
  (`AbilityTask_PlayMontageAndWait.CreatePlayMontageAndWaitProxy` "None" (`WeaponStaticData.AttackMontage` (`self.GetEquippedItemWeaponStaticData`))
    (:`then`
      (bind _returnvalue (`KismetSystemLibrary.K2_SetTimerDelegate` (delegate `Shoot`) (/ 1.0 (`WeaponStaticData.FireRate` (`self.GetEquippedItemWeaponStaticData`))) true))
      (set `self.ShootTimerHandle` _returnvalue)
      (`self.Shoot`)
      (`AbilityTask_WaitGameplayEvent.WaitGameplayEvent` (struct :`TagName` "Event.Combat.Attack.Ended") null true
        (:`EventReceived`
          (`self.K2_EndAbility`))))
    (:`OnCompleted`
      (`self.K2_EndAbility` :!label _label))
    (:`OnInterrupted`
      (goto _label))
    (:`OnCancelled`
      (goto _label))))

(event `Shoot`
  (bind _returnvalue (`WeaponItemActor.GetMuzzleLocation` (`self.GetEquippedWeaponItemActor`)))
  (bind (_outhit _returnvalue_2) (`KismetSystemLibrary.LineTraceSingle` :`Start` _returnvalue :`End` (+ _returnvalue (* (`Controller.GetControlRotation` (`.PlayerController` (break `GameplayAbilityActorInfo` (`self.GetActorInfo`)))) (`self.ShootingDistance`))) :`TraceChannel` "TraceTypeQuery1" :`DrawDebugType` "ForDuration"))
  (if _returnvalue_2
    (bind _returnvalue_3 (`AbilitySystemBlueprintLibrary.GetAbilitySystemComponent` (`.HitActor` (`GameplayStatics.BreakHitResult` _outhit))))
    (`/Engine/EditorBlueprintResources/StandardMacros.IsValid` _returnvalue_3
      (:`Is Valid`
        (`AbilitySystemComponent.BP_ApplyGameplayEffectToSelf` :`self` _returnvalue_3 :`GameplayEffectClass` (`WeaponStaticData.DamageEffect` (`self.GetEquippedItemWeaponStaticData`)))))))

(event `self.K2_OnEndAbility`
  (params (bWasCancelled :type Boolean))
  (`KismetSystemLibrary.K2_ClearAndInvalidateTimerHandle` (`self.ShootTimerHandle`)))